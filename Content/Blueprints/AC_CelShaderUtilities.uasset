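; Actor component that drives cel-shader lighting parameters on its owner's materials from a chosen light source or, optionally, the first directional light found.
; AddComponent creates and registers dynamic material instances for given slots.
; Each tick, an optional line trace toward the light detects shadowing, smoothly fading the Light parameter.
; Light direction (rotation- or position-based), color and ambient color update on SetLightSource, or every tick for dynamic sources.
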(event EventBeginPlay
  (if (Variables|Default|General|GetUseDirectionalLightAsDefaultLightSource)
    (bind _outactors (Actor|GetAllActorsOfClass "/Script/Engine.DirectionalLight"))
    (if (Utilities|Array|IsValidIndex _outactors)
      (Variables|Default|LightSource|SetLightSource (Utilities|Array|Get(acopy) _outactors)))))

(event EventTick
  (params (DeltaSeconds :type Float%20%28single-precision%29))
  (CallFunction|Trace)
  (CallFunction|UpdateLightValue DeltaSeconds)
  (if (Variables|Default|LightSource|GetDynamicLightSource)
    (CallFunction|UpdateLightSourceValues)))

(fn AddComponent
  (params (Component :type Primitive%20Component%20Object%20Reference) (Slots :type Array%20of%20Integers))
  (for _array_element Slots
    (bind _returnvalue (Rendering|Material|CreateDynamicMaterialInstance Component _array_element (Rendering|Material|GetMaterial Component _array_element) "None" :!class /Script/Engine.PrimitiveComponent))
    (Utilities|Map|Add (Variables|Ref|GetDynamicMaterials) _returnvalue Component)))

(fn Trace
  (bind _returnvalue (Components|GetOwner))
  (bind _returnvalue_2 (Transformation|GetActorLocation _returnvalue))
  (if (Variables|Default|Tracing|GetEnableTracing)
    (Utilities|IsValid (Variables|Default|LightSource|GetLightSource)
      (:Is%20Valid
        (bind _returnvalue_3 (Collision|LineTraceByChannel _returnvalue_2 (+ _returnvalue_2 (Variables|State|GetLightDirection)) (Variables|Default|Tracing|GetTraceChannel) false 0 "None"))
        (Variables|State|SetLit (not _returnvalue_3))))))

(fn UpdateLightValue
  (params (DeltaTime :type Float%20%28double-precision%29))
  (bind _keys (Utilities|Map|Keys (Variables|Ref|GetDynamicMaterials)))
  (for _array_element _keys
    (bind _returnvalue (Rendering|Material|GetScalarParameterValue _array_element "Light" :!class /Script/Engine.MaterialInstanceDynamic))
    (Rendering|Material|SetScalarParameterValue _array_element "Light" (Math|Interpolation|FInterpTo _returnvalue (* (Math|Float|SelectFloat 1.0 0.0 (Variables|State|GetLit)) (Variables|Default|General|GetBrightness) (Variables|State|GetLightBrightness)) DeltaTime 1e+01) :!class /Script/Engine.MaterialInstanceDynamic)))

(fn UpdateLightSourceValues
  (Utilities|IsValid (Variables|Default|LightSource|GetLightSource)
    (:Is%20Valid
      (Variables|State|SetLightDirection (Math|Vector|SelectVector (* (* (Transformation|GetActorForwardVector (Variables|Default|LightSource|GetLightSource)) -1.0) (Variables|Default|Tracing|GetTraceLength)) (* (Math|Vector|Normalize (- (Transformation|GetActorLocation (Variables|Default|LightSource|GetLightSource)) (Transformation|GetActorLocation (Components|GetOwner)))) (Variables|Default|Tracing|GetTraceLength)) (Variables|Default|LightSource|GetLightSourceIsDirectionOnly)))
      ;[1 1 1] Fetching light source parameters
      (bind _aslight (Utilities|Casting|CastToLight (Variables|Default|LightSource|GetLightSource))
        (:then
          (Variables|State|SetLightColor (Rendering|Components|Light|GetLightColor (Variables|/Script/Engine.Light|GetLightComponent _aslight)))
          (Variables|State|SetLightBrightness (/ (Variables|/Script/Engine.LightComponentBase|GetIntensity (Variables|/Script/Engine.Light|GetLightComponent _aslight)) 8.0)))
        (:CastFailed
          (Variables|State|SetLightColor "(R=1.000000,G=1.000000,B=1.000000,A=1.000000)")
          (Variables|State|SetLightBrightness 1.0)))
      (if (Variables|Default|General|LightColorOverride|GetOverrideLightColor)
        (Variables|State|SetLightColor (Variables|Default|General|LightColorOverride|GetLightColorOverride)))
      (bind _keys (Utilities|Map|Keys (Variables|Ref|GetDynamicMaterials)))
      (for _array_element _keys
        (Rendering|Material|SetVectorParameterValue _array_element "CustomLightDireciton" (Math|Conversions|ToLinearColor(Vector) (Variables|State|GetLightDirection)) :!class /Script/Engine.MaterialInstanceDynamic)
        (Rendering|Material|SetVectorParameterValue _array_element "LightColor" (Variables|State|GetLightColor) :!class /Script/Engine.MaterialInstanceDynamic)
        (Rendering|Material|SetVectorParameterValue _array_element "AmbientLightColor" (Variables|Default|General|GetAmbientLightColor) :!class /Script/Engine.MaterialInstanceDynamic)))))

(fn SetLightSource
  (params (LightSource :type Actor%20Object%20Reference) (DynamicLightSource :type Boolean) (LightSourceIsDirectionOnly :type Boolean))
  (Variables|Default|LightSource|SetLightSource LightSource)
  (Variables|Default|LightSource|SetDynamicLightSource DynamicLightSource)
  (Variables|Default|LightSource|SetLightSourceIsDirectionOnly LightSourceIsDirectionOnly)
  (CallFunction|UpdateLightSourceValues))