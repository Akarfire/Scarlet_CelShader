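; Actor component that detects whether its owner is in direct light or shadow and feeds the result to cel-shader materials.
; On BeginPlay it finds a tagged directional light, then each Tick line-traces from the owner against the light's direction to set Lit.
; AddComponent registers mesh slots as dynamic material instances, whose "Light" scalar is smoothly interpolated toward 1 when lit and 0 when blocked.
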(event EventBeginPlay
  (bind _outactors (Actor|GetAllActorsOfClasswithTag "/Script/Engine.DirectionalLight" "M"))
  (if (Utilities|Array|IsValidIndex _outactors)
    (Variables|Default|SetDirectionalLight (Utilities|Array|Get(acopy) _outactors))))

(event EventTick
  (params (DeltaSeconds :type Float%20%28single-precision%29))
  (CallFunction|Trace)
  (CallFunction|UpdateLightValue DeltaSeconds))

(fn AddComponent
  (params (Component :type Primitive%20Component%20Object%20Reference) (Slots :type Array%20of%20Integers))
  (for _array_element Slots
    (bind _returnvalue (Rendering|Material|CreateDynamicMaterialInstance Component _array_element (Rendering|Material|GetMaterial Component _array_element) "None" :!class /Script/Engine.PrimitiveComponent))
    (Utilities|Map|Add (Variables|Default|GetDynamicMaterials) _returnvalue Component)))

(fn Trace
  (bind _returnvalue (Components|GetOwner))
  (bind _returnvalue_2 (Transformation|GetActorLocation _returnvalue))
  (Utilities|IsValid (Variables|Default|GetDirectionalLight)
    (:Is%20Valid
      (bind _returnvalue_3 (Collision|LineTraceByChannel _returnvalue_2 (+ _returnvalue_2 (* (* (Transformation|GetActorForwardVector (Variables|Default|GetDirectionalLight)) -1.0) (Variables|Default|GetTraceLenght))) "TraceTypeQuery1" false 0 "None"))
      (Variables|Default|SetLit (not _returnvalue_3)))))

(fn UpdateLightValue
  (params (DeltaTime :type Float%20%28double-precision%29))
  (bind _keys (Utilities|Map|Keys (Variables|Default|GetDynamicMaterials)))
  (for _array_element _keys
    (bind _returnvalue (Rendering|Material|GetScalarParameterValue _array_element "Light" :!class /Script/Engine.MaterialInstanceDynamic))
    (Rendering|Material|SetScalarParameterValue _array_element "Light" (Math|Interpolation|FInterpTo _returnvalue (Math|Float|SelectFloat 1.0 0.0 (Variables|Default|GetLit)) DeltaTime 1e+01) :!class /Script/Engine.MaterialInstanceDynamic)))